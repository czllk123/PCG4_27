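; Hierarchical scatter actor that places random static meshes in nested radial layers from its construction script.
; Each SpawnerConfig layer spreads points at even angles and random radii, using the previous layer's points as centers.
; An optional line trace adjusts height and blends rotation toward the surface normal.
; Pre-trace transforms and meshes are stored, so FreezeArrangement rebuilds the same layout and re-traces it instead of regenerating.
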(fn ConstructionScript
  (Utilities|FlowControl|Sequence
    (:then_0
      (if (Variables|SpawnerConfig|GetFreezeArrangement)
        (CallFunction|SpawnFrozenArrangement)
        (else
          (if (Variables|SpawnerConfig|GetRandomize)
            (Variables|SpawnerConfig|SetRandomize false))
          (CallFunction|Generate))))))

(fn SpawnFrozenArrangement
  (Utilities|Array|Clear (Variables|SpawnerConfig|DONOTTOUCH|GetStoredSpawns_PostTrace))
  ;[0 0 0] Spwan frozen transforms and meshes
  (for _array_element (Variables|SpawnerConfig|DONOTTOUCH|GetStoredSpawns)
    (bind _returnvalue (AddComponent|AddStaticMeshComponent false (.pointlocations _array_element)))
    (LocalVariables|SetSpawnedComponent _returnvalue)
    (Components|StaticMesh|SetStaticMesh (LocalVariables|GetSpawnedComponent) (.mesh _array_element))
    ;[0 0 0] Trace during generation
    (if (Variables|TraceSettings|GetEnableTrace?)
      (bind (_newlocation _newrotation) (CallFunction|GetTracedTransformforPoint (.Location (Math|Transform|BreakTransform (Transformation|GetRelativeTransform (LocalVariables|GetSpawnedComponent)))) (.Rotation (Math|Transform|BreakTransform (Transformation|GetRelativeTransform (LocalVariables|GetSpawnedComponent))))))
      (Transformation|SetRelativeTransform (LocalVariables|GetSpawnedComponent) (Math|Transform|MakeTransform _newlocation _newrotation (.Scale (Math|Transform|BreakTransform (Transformation|GetRelativeTransform (LocalVariables|GetSpawnedComponent))))) false false)
      (Utilities|Array|Add (Variables|SpawnerConfig|DONOTTOUCH|GetStoredSpawns_PostTrace) (Utilities|Struct|MakeST_StoredSpawns (Transformation|GetRelativeTransform (LocalVariables|GetSpawnedComponent)) (Variables|/Script/Engine.StaticMeshComponent|GetStaticMesh (LocalVariables|GetSpawnedComponent)))))))

(fn GetTracedTransformforPoint
  (params (Point%20Location :type Vector) (Point%20Rotation :type Rotator))
  (bind _returnvalue (Transformation|GetActorTransform))
  (bind _returnvalue_2 (Math|Transform|TransformLocation _returnvalue Point%20Location))
  (bind _outhit (Collision|LineTraceByChannel _returnvalue_2 (+ _returnvalue_2 (Math|Vector|MakeVector 0.0 0.0 (Variables|TraceSettings|GetTraceDistance))) "TraceTypeQuery1" false (Variables|TraceSettings|GetActors%20to%20Ignore) "None" true "(R=1.000000,G=0.000000,B=0.000000,A=1.000000)" "(R=0.000000,G=1.000000,B=0.000000,A=1.000000)" 1.0))
  ;[0 0 0] Final Location of the point
  (LocalVariables|SetModifiedLocation (+ Point%20Location (Math|Vector|MakeVector 0.0 0.0 (.Z (Math|Vector|BreakVector (Math|Transform|InverseTransformLocation (Transformation|GetActorTransform) (.Location (Collision|BreakHitResult _outhit))))))))
  ;[0 0 0] Final rotation
  (LocalVariables|SetModifiedRotation (Math|Rotator|Lerp(Rotator) Point%20Rotation (Math|Rotator|SelectRotator (Math|Rotator|MakeRotator (.roll (Math|Rotator|MakeRotfromXZ (Math|Vector|GetForwardVector Point%20Rotation) (.ImpactNormal (Collision|BreakHitResult _outhit)))) (.pitch (Class|KismetMathLibrary|MakeRotfromYZ (Math|Vector|GetRightVector Point%20Rotation) (.ImpactNormal (Collision|BreakHitResult _outhit)))) (.Yaw (Math|Rotator|BreakRotator Point%20Rotation))) Point%20Rotation (Variables|TraceSettings|GetAlignToNormal)) (Variables|TraceSettings|GetMatchNormalRatio)))
  (return (LocalVariables|GetModifiedLocation) (LocalVariables|GetModifiedRotation)))

(fn Generate
  ;[0 0 0] Cleanup and reset vars if required
  (CallFunction|Cleanup)
  (CallFunction|LayerdSpawner))

(fn Cleanup
  (Utilities|Array|Clear (Variables|SpawnerConfig|DONOTTOUCH|GetStoredSpawns))
  (Utilities|Map|Clear (Variables|SpawnerConfig|GetGeneratedSpawnPoints))
  (Utilities|Array|Clear (Variables|SpawnerConfig|DONOTTOUCH|GetStoredSpawns_PostTrace)))

(fn LayerdSpawner
  (for (_array_element _array_index) (Variables|SpawnerConfig|GetSpawnerConfig)
    (if (== _array_index 0)
      (bind _generatedspawnpoints (CallFunction|Spawner (.ScatterCounts (Utilities|Struct|BreakST_LayerSettring _array_element)) (.MinMaxRadius (Utilities|Struct|BreakST_LayerSettring _array_element)) (.Mesh (Utilities|Struct|BreakST_LayerSettring _array_element)) "0, 0, 0" (.RandZRotation (Utilities|Struct|BreakST_LayerSettring _array_element))))
      (Utilities|Map|Add (Variables|SpawnerConfig|GetGeneratedSpawnPoints) 0 (Utilities|Struct|MakeST_SpawnPoints _generatedspawnpoints))
      (else
        (CallFunction|SpawnerforNextLayers (.ScatterCounts (Utilities|Struct|BreakST_LayerSettring _array_element)) (.MinMaxRadius (Utilities|Struct|BreakST_LayerSettring _array_element)) (.Mesh (Utilities|Struct|BreakST_LayerSettring _array_element)) _array_index (.RandZRotation (Utilities|Struct|BreakST_LayerSettring _array_element)))))))

(fn Spawner
  (params (Segments :type Integer) (Radius :type Vector%202D%20Structure) (NewMesh :type Array%20of%20ST%20Per%20Mesh%20Setting%20Structures) (ReferencePoint :type Vector) (RandRotation :type Vector%202D%20Structure))
  (bind (_x _y) (Math|Vector2D|BreakVector2D RandRotation))
  ;[0 0 0] Random radius of distribution per point
  (LocalVariables|SetAnglePerSegment (/ 360 Segments))
  (for _index (range 0 (- Segments 1))
    (LocalVariables|SetCurrentIndex _index)
    (LocalVariables|SetRandRadius (Math|Random|RandomFloatinRange (.x Radius) (.y Radius)))
    (LocalVariables|SetGeneratedSpawnPoint (+ ReferencePoint (* (Math|Vector|GetForwardVector (Math|Rotator|MakeRotator 0.0 0.0 (Math|Conversions|ToFloat(Integer) (* (LocalVariables|GetCurrentIndex) (LocalVariables|GetAnglePerSegment))))) (LocalVariables|GetRandRadius))))
    ;[0 0 0] Randome mesh rotation
    (LocalVariables|SetRandomedRotation (Math|Rotator|MakeRotator 0.0 0.0 (Math|Random|RandomFloatinRange _x _y)))
    (Utilities|Array|Add (LocalVariables|GetSpawnPoints) (LocalVariables|GetGeneratedSpawnPoint)) ; Store generated points for freeze functionality
    ;[0 0 0] Create and assign random static mesh at generated location and rotation
    (bind _output_get (LocalVariables|SetCurrentMeshItem (.OutItem (Utilities|Array|Random NewMesh))))
    (Utilities|IsValid (Utilities|Struct|BreakST_PerMeshSetting _output_get)
      (:Is%20Valid
        (bind _returnvalue (AddComponent|AddStaticMeshComponent false (Math|Transform|MakeTransform (LocalVariables|GetGeneratedSpawnPoint) (LocalVariables|GetRandomedRotation) (Math|Conversions|ToVector(Float) (Math|Random|RandomFloatinRange (.x (.RandScale (Utilities|Struct|BreakST_PerMeshSetting (LocalVariables|GetCurrentMeshItem)))) (.y (.RandScale (Utilities|Struct|BreakST_PerMeshSetting (LocalVariables|GetCurrentMeshItem)))))))))
        (LocalVariables|SetCreatedComponent _returnvalue)
        (LocalVariables|SetRandomedMesh (.Mesh (Utilities|Struct|BreakST_PerMeshSetting (LocalVariables|GetCurrentMeshItem))))
        (Components|StaticMesh|SetStaticMesh (LocalVariables|GetCreatedComponent) (LocalVariables|GetRandomedMesh))
        (Utilities|Array|Add (Variables|SpawnerConfig|DONOTTOUCH|GetStoredSpawns) (Utilities|Struct|MakeST_StoredSpawns (Transformation|GetRelativeTransform (LocalVariables|GetCreatedComponent)) (LocalVariables|GetRandomedMesh)))
        ;[0 0 0] Trace during generation
        (if (Variables|TraceSettings|GetEnableTrace?)
          (bind (_newlocation _newrotation) (CallFunction|GetTracedTransformforPoint (.Location (Math|Transform|BreakTransform (Transformation|GetRelativeTransform (LocalVariables|GetCreatedComponent)))) (.Rotation (Math|Transform|BreakTransform (Transformation|GetRelativeTransform (LocalVariables|GetCreatedComponent))))))
          (Transformation|SetRelativeLocation (LocalVariables|GetCreatedComponent) _newlocation false false)
          (Transformation|SetRelativeRotation (LocalVariables|GetCreatedComponent) _newrotation false false)
          (Utilities|Array|Add (Variables|SpawnerConfig|DONOTTOUCH|GetStoredSpawns_PostTrace) (Utilities|Struct|MakeST_StoredSpawns (Transformation|GetRelativeTransform (LocalVariables|GetCreatedComponent)) (Variables|/Script/Engine.StaticMeshComponent|GetStaticMesh (LocalVariables|GetCreatedComponent))))))))
  (return (LocalVariables|GetSpawnPoints)))

(fn SpawnerforNextLayers
  (params (Segments :type Integer) (Radius :type Vector%202D%20Structure) (NewMesh :type Array%20of%20ST%20Per%20Mesh%20Setting%20Structures) (CurrentLayerIndex :type Integer%20%28by%20ref%29) (RandRotation :type Vector%202D%20Structure))
  (Utilities|Array|Clear (LocalVariables|GetTempArray))
  (for _array_element (.points (.Value (Utilities|Map|Find (Variables|SpawnerConfig|GetGeneratedSpawnPoints) (- CurrentLayerIndex 1))))
    (bind _generatedspawnpoints (CallFunction|Spawner Segments Radius NewMesh (Math|Vector|MakeVector (.x _array_element) (.y _array_element) 0.0) RandRotation))
    (Utilities|Array|AppendArray (LocalVariables|GetTempArray) _generatedspawnpoints))
  (Utilities|Map|Add (Variables|SpawnerConfig|GetGeneratedSpawnPoints) CurrentLayerIndex (Utilities|Struct|MakeST_SpawnPoints (LocalVariables|GetTempArray)))
  (return))